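; BP_TalkableNPC is an NPC that opens a dialogue widget when interacted with.
; Its Interaction event creates WBP_Dialogue with the NPC's dialogue lines, adds it to the viewport and gives it keyboard focus, while interface-style getters report an interaction method and zero hold time.
; A box collider tracks whether the first-person character is in range, but that flag only drives right-mouse debug prints.
; A StartCombat call on the game mode is left unconnected.
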(event `self.ReceiveBeginPlay`
  (`self.EnableInput` (`GameplayStatics.GetPlayerController` 0)))

(event `self.BoxCollider.OnComponentBeginOverlap`
  (params (OverlappedComponent :type "PrimitiveComponent Object Reference") (OtherActor :type "Actor Object Reference") (OtherComp :type "PrimitiveComponent Object Reference") (OtherBodyIndex :type Integer) (bFromSweep :type Boolean) (SweepResult :type "HitResult Structure (by ref)"))
  (cast `/Game/FirstPerson/Blueprints/BP_FirstPersonCharacter` OtherActor)
  (set `self.PlayerinRange` true))

(event `self.BoxCollider.OnComponentEndOverlap`
  (params (OverlappedComponent :type "PrimitiveComponent Object Reference") (OtherActor :type "Actor Object Reference") (OtherComp :type "PrimitiveComponent Object Reference") (OtherBodyIndex :type Integer))
  (cast `/Game/FirstPerson/Blueprints/BP_FirstPersonCharacter` OtherActor)
  (set `self.PlayerinRange` false))

(event `/Game/Roberts_stuff/LevelPrototyping/Interactable/Interaction_manager/BPI_interacble.Interaction`
  (params (Interactor :type "Actor Object Reference"))
  (bind _returnvalue (`|CreateWidget` "/Game/NPCs/WBP_Dialogue.WBP_Dialogue_C" (`GameplayStatics.GetPlayerController` 0) (`self.DialogueSwitch`)))
  (bind _output_get (set `self.DialogueWidget` _returnvalue))
  (`UserWidget.AddToViewport` _output_get 0)
  (`Widget.SetKeyboardFocus` _returnvalue))

(event `Key|RightMouseButton`
  (params (Key :type "Key Structure"))
  (:`Pressed`
    (`KismetSystemLibrary.PrintString` "RMB Pressed")
    (if (`self.PlayerinRange`)
      (`KismetSystemLibrary.PrintString` "In Range")
      (else
        (`KismetSystemLibrary.PrintString` "No")))))

(fn `GetInteractionMethod`
  (returns (`Interact Method` :type "/Game/Roberts_stuff/LevelPrototyping/Interactable/Interaction_manager/Interaction_Method Enum"))
  (return "NewEnumerator0"))

(fn `holdTime`
  (returns (Time :type "Float (double-precision)"))
  (return 0.0))

(fn `UserConstructionScript`)