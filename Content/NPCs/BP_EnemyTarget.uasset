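; Enemy NPC with melee and ranged attacks that rolls a random type on BeginPlay, with one type randomizing among four shooter stat presets.
; Melee and Shoot update an overhead label, then play range-gated montages.
; DoPunch sphere-traces to hit the player, ShootGun spawns player-aimed bullets, and Finish events reset attack flags.
; Damage flashes the mesh red before reducing Health; death notifies the wave manager and destroys the actor.
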(event `self.ReceiveBeginPlay`
  (`KismetSystemLibrary.PrintString` (`KismetStringLibrary.Conv_DoubleToString` (`self.Health`)))
  (`|ExecutionSequence`
    (:`then_0`
      (`KismetSystemLibrary.PrintString` "beginning play")
      (set `self.HomeLocation` (`self.K2_GetActorLocation`))
      (set `self.EnemyType` (`KismetMathLibrary.RandomIntegerInRange` 0 2))
      (set `self.CanAttack` true))
    (:`then_1`
      (bind _returnvalue (`PrimitiveComponent.CreateDynamicMaterialInstance` (`self.Mesh`) 0 null "None"))
      (set `self.EnemyDefaultMaterial1` _returnvalue))
    (:`then_2`
      (bind _returnvalue_2 (`PrimitiveComponent.CreateDynamicMaterialInstance` (`self.Mesh`) 1 null "None"))
      (set `self.EnemyDefaultMaterial2` _returnvalue_2))
    (:`then_3`
      (if (== (`self.EnemyType`) 2)
        (`self.SetupShooterType`)
        (`KismetSystemLibrary.PrintString` "ShooterTypeCall Read")))
    (:`then_4`
      (bind _aswbp_enemy_label (cast `/Game/NPCs/WBP_EnemyLabel` (`WidgetComponent.GetUserWidgetObject` (`self.EnemyLabel`))))
      (`/Game/NPCs/WBP_EnemyLabel.SetEnemyLabel` _aswbp_enemy_label "Walk"))))

(event `Melee`
  (bind _aswbp_enemy_label (cast `/Game/NPCs/WBP_EnemyLabel` (`WidgetComponent.GetUserWidgetObject` (`self.EnemyLabel`))))
  (`/Game/NPCs/WBP_EnemyLabel.SetEnemyLabel` _aswbp_enemy_label "Melee")
  (if (and (<= (`self.GetDistanceTo` (`GameplayStatics.GetPlayerCharacter` 0)) (`self.MaxMeleeRange`)) (not (`self.IsAttacking`)) (`self.CanAttack`) (`self.CanMelee`))
    (`KismetSystemLibrary.PrintString` "Punch Anim meant to play")
    (set `self.IsAttacking` true)
    (set `self.CanAttack` true)
    (set `self.isWalking` false)
    (set `self.DetectRange` 1500.0)
    (`MovementComponent.StopMovementImmediately` (`self.CharacterMovement`))
    (`self.PlayAnimMontage` "/Game/NPCs/anim/AM_Punch.AM_Punch")
    (`KismetSystemLibrary.PrintString` "Start Punch")))

(event `Shoot`
  (bind _aswbp_enemy_label (cast `/Game/NPCs/WBP_EnemyLabel` (`WidgetComponent.GetUserWidgetObject` (`self.EnemyLabel`))))
  (`/Game/NPCs/WBP_EnemyLabel.SetEnemyLabel` _aswbp_enemy_label "Shoot")
  (if (and (<= (`self.GetDistanceTo` (`GameplayStatics.GetPlayerCharacter` 0)) (`self.MaxShootRange`)) (not (`self.IsAttacking`)) (`Controller.LineOfSightTo` (`self.GetController`) (`GameplayStatics.GetPlayerCharacter` 0) (0.0 0.0 0.0) false) (`self.CanAttack`) (>= (`self.GetDistanceTo` (`GameplayStatics.GetPlayerCharacter` 0)) (`self.MinShootRange`)) (`self.CanShoot`))
    (set `self.IsAttacking` true)
    (set `self.CanAttack` false)
    (set `self.isWalking` false)
    (`MovementComponent.StopMovementImmediately` (`self.CharacterMovement`))
    (`self.PlayAnimMontage` "/Game/NPCs/anim/RifleMontage.RifleMontage")))

(event `ShootGun`
  (`|SpawnActorFromClass` "/Game/NPCs/BP_Bullet.BP_Bullet_C" (`KismetMathLibrary.MakeTransform` (`SceneComponent.K2_GetComponentLocation` (`self.FirePoint`)) (`KismetMathLibrary.FindLookAtRotation` (`SceneComponent.K2_GetComponentLocation` (`self.FirePoint`)) (`self.K2_GetActorLocation` (`GameplayStatics.GetPlayerCharacter` 0)))) "Undefined" "MultiplyWithRoot" null null)
  (`KismetSystemLibrary.PrintString` "Fire")
  (`KismetSystemLibrary.Delay` (`self.FireRate`)))

(event `DoShoot`
  (`self.ShootGun`))

(event `FinishShoot`
  (set `self.IsAttacking` false)
  (set `self.CanAttack` true))

(event `EnemyTakeDamage`
  (params (DamageAmount :type "Float (double-precision)" :default 1.0))
  (`self.ProcessEnemyDamage` DamageAmount))

(event `self.ReceiveAnyDamage`
  (params (Damage :type "Float (single-precision)") (DamageType :type "DamageType Object Reference") (InstigatedBy :type "Controller Object Reference") (DamageCauser :type "Actor Object Reference"))
  (`self.ProcessEnemyDamage` Damage))

(event `Death`
  (`KismetSystemLibrary.PrintString` "ENEMY DEAD")
  (`/Game/NPCs/BP_WaveManager.EnemyDeath` (`self.WaveManagerRef`))
  (`self.K2_DestroyActor`))

(event `StopToAttack`
  (bind _charactermovement (`self.CharacterMovement`))
  (if (<= (`self.GetDistanceTo` (`GameplayStatics.GetPlayerCharacter` 0)) (`self.StopRange`))
    (set `CharacterMovementComponent.MaxWalkSpeed` 50.0 _charactermovement)
    (else
      (set `CharacterMovementComponent.MaxWalkSpeed` 600.0 _charactermovement))))

(event `DoPunch`
  (bind (_outhit _returnvalue) (`KismetSystemLibrary.SphereTraceSingle` (`self.K2_GetActorLocation`) (+ (`self.K2_GetActorLocation`) (* (`self.GetActorForwardVector`) 120.0)) 45.0 "TraceTypeQuery3"))
  (if _returnvalue
    (bind _asbp_first_person_character (cast `/Game/FirstPerson/Blueprints/BP_FirstPersonCharacter` (`.HitActor` (`GameplayStatics.BreakHitResult` _outhit))))
    (`/Game/FirstPerson/Blueprints/BP_FirstPersonCharacter.Hit` _asbp_first_person_character 1.0)
    (`KismetSystemLibrary.PrintString` "Punch Hit Activated")))

(event `Finish Punch`
  (`KismetSystemLibrary.Delay` 0.8)
  (set `self.IsAttacking` false)
  (set `self.CanAttack` true)
  (if (<= (`self.GetDistanceTo` (`GameplayStatics.GetPlayerCharacter` 0)) (`self.MaxMeleeRange`))
    (`self.Melee`)))

(event `SetupShooterType`
  (bind _returnvalue (`KismetMathLibrary.RandomIntegerInRange` 0 3))
  (`KismetSystemLibrary.PrintString` (`KismetStringLibrary.Conv_IntToString` _returnvalue))
  (switch `int` _returnvalue
    (:`0`
      (`KismetSystemLibrary.PrintString` "Basic Shooter")
      (set `self.MaxShootRange` 300.0)
      (set `self.MinShootRange` 100.0)
      (set `self.FireRate` 1.0)
      (set `self.Health` 3.0)
      (set `self.DetectRange` 450.0))
    (:`1`
      (`KismetSystemLibrary.PrintString` "Long Range Shooter")
      (set `self.MaxShootRange` 1000.0)
      (set `self.MinShootRange` 200.0)
      (set `self.FireRate` 1.2)
      (set `self.Health` 3.0)
      (set `self.DetectRange` 1200.0))
    (:`2`
      (`KismetSystemLibrary.PrintString` "Weak Enemy")
      (set `self.MaxShootRange` 1500.0)
      (set `self.MinShootRange` 70.0)
      (set `self.FireRate` 1.5)
      (set `self.Health` 1.0)
      (set `self.DetectRange` 1700.0))
    (:`3`
      (`KismetSystemLibrary.PrintString` "Tank Shooter")
      (set `self.MaxShootRange` 300.0)
      (set `self.MinShootRange` 100.0)
      (set `self.FireRate` 0.5)
      (set `self.Health` 6.0)
      (set `self.DetectRange` 450.0))))

(event `ProcessEnemyDamage`
  (params (Damage :type "Float (double-precision)"))
  (`MeshComponent.SetVectorParameterValueOnMaterials` (`self.Mesh`) "Paint Tint" (1.0 0.0 0.0))
  (`KismetSystemLibrary.Delay` 0.3)
  (`MeshComponent.SetVectorParameterValueOnMaterials` (`self.Mesh`) "Paint Tint" (1.0 1.0 1.0))
  (bind _output_get (set `self.Health` (- (`self.Health`) Damage)))
  (if (<= _output_get 0.0)
    (`self.Death`)))

(fn `UserConstructionScript`)