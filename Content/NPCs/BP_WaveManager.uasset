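; Wave manager actor that runs enemy waves with a countdown before each, tracked by two HUD widgets.
; StartWave removes talkable NPCs and starts a looping one-second timer, which spawns BP_EnemyTarget at random spawn points using per-wave counts.
; EnemyDeath updates the remaining count; at zero it advances the wave, restarts the countdown and toggles BP_DoorFrame's EnemysDead flag.
; Passing MaxWaves sets WaveComplete, but the countdown still restarts.
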(event `self.ReceiveBeginPlay`
  (bind _enemiesremainingref (`self.EnemiesRemainingRef`))
  (bind _returnvalue (`|CreateWidget` "/Game/NPCs/WBP_Countdown.WBP_Countdown_C" (`GameplayStatics.GetPlayerController` 0)))
  (bind _output_get (set `self.CountdownRef` _returnvalue))
  (`UserWidget.AddToViewport` _output_get 0)
  (`Widget.SetVisibility` (`self.CountdownRef`) "Hidden")
  (bind _returnvalue_2 (`|CreateWidget` "/Game/NPCs/WBP_EnemiesRemaining.WBP_EnemiesRemaining_C" (`GameplayStatics.GetPlayerController` 0)))
  (set `self.EnemiesRemainingRef` _returnvalue_2)
  (`UserWidget.AddToViewport` _enemiesremainingref 0)
  (`Widget.SetVisibility` _enemiesremainingref "Hidden"))

(event `StartWave`
  (bind _returnvalue (`GameplayStatics.GetActorOfClass` "/Game/Roberts_stuff/LevelPrototyping/Interactable/Door/BP_DoorFrame.BP_DoorFrame_C"))
  (set `/Game/Roberts_stuff/LevelPrototyping/Interactable/Door/BP_DoorFrame.Enemy's Dead?` false _returnvalue)
  (`Widget.SetVisibility` (`self.EnemiesRemainingRef`) "Visible")
  (`KismetSystemLibrary.PrintString` "Wave 1")
  (set `self.CurrentWave` 0)
  (set `self.WaveComplete` false)
  (`self.StartNextWave`)
  (`self.StartCountdown`)
  (bind _outactors (`GameplayStatics.GetAllActorsOfClass` "/Game/NPCs/BP_TalkableNPC.BP_TalkableNPC_C"))
  (`self.K2_DestroyActor` _outactors))

(event `StartNextWave`
  (set `self.TimeUntilNextWave` 15)
  (set `self.CurrentWave` (+ (`self.CurrentWave`) 1))
  (if (not (<= (`self.CurrentWave`) (`self.MaxWaves`)))
    (set `self.WaveComplete` true)))

(event `SpawnCurrentWave`
  (bind _spawnpoints (`self.SpawnPoints`))
  (bind _output_get (set `self.EnemiesAlive` (`|GetArrayItem` (`self.MaxWaveEnemyCount`) (- (`self.CurrentWave`) 1))))
  (`/Game/NPCs/WBP_EnemiesRemaining.SetEnemiesRemainingText` (`self.EnemiesRemainingRef`) (`self.EnemiesAlive`))
  (for _ (range _output_get)
    (bind _returnvalue (`|SpawnActorFromClass` "/Game/NPCs/BP_EnemyTarget.BP_EnemyTarget_C" (`self.GetTransform` (`|GetArrayItem` _spawnpoints (`KismetMathLibrary.RandomIntegerInRange` 0 (- (`KismetArrayLibrary.Array_Length` _spawnpoints) 1)))) "AlwaysSpawn" "MultiplyWithRoot" null null))
    (set `/Game/NPCs/BP_EnemyTarget.WaveManagerRef` self _returnvalue)))

(event `EnemyDeath`
  (bind _output_get (set `self.EnemiesAlive` (- (`self.EnemiesAlive`) 1)))
  (`/Game/NPCs/WBP_EnemiesRemaining.SetEnemiesRemainingText` (`self.EnemiesRemainingRef`) _output_get)
  (if (<= (`self.EnemiesAlive`) 0)
    (`self.StartNextWave`)
    (`self.StartCountdown`)
    (bind _returnvalue (`GameplayStatics.GetActorOfClass` "/Game/Roberts_stuff/LevelPrototyping/Interactable/Door/BP_DoorFrame.BP_DoorFrame_C"))
    (set `/Game/Roberts_stuff/LevelPrototyping/Interactable/Door/BP_DoorFrame.Enemy's Dead?` true _returnvalue)))

(event `StartCountdown`
  (bind _countdownref (`self.CountdownRef`))
  (set `self.WaveCountdown` (`self.TimeUntilNextWave`))
  (`Widget.SetVisibility` _countdownref "Visible")
  (`/Game/NPCs/WBP_Countdown.SetCountdownText` _countdownref (`self.TimeUntilNextWave`))
  (bind _returnvalue (`KismetSystemLibrary.K2_SetTimerDelegate` (`|CreateDelegate` :!event `UpdateCountdown`) 1.0 true))
  (set `self.CountdownTimerHandle` _returnvalue))

(event `UpdateCountdown`
  (bind _output_get (set `self.TimeUntilNextWave` (- (`self.TimeUntilNextWave`) 1)))
  (`/Game/NPCs/WBP_Countdown.SetCountdownText` (`self.CountdownRef`) _output_get)
  (if (<= (`self.TimeUntilNextWave`) 0)
    (`Widget.SetVisibility` (`self.CountdownRef`) "Hidden")
    (`KismetSystemLibrary.K2_ClearAndInvalidateTimerHandle` (`self.CountdownTimerHandle`))
    (`self.SpawnCurrentWave`)
    (bind _returnvalue (`GameplayStatics.GetActorOfClass` "/Game/Roberts_stuff/LevelPrototyping/Interactable/Door/BP_DoorFrame.BP_DoorFrame_C"))
    (set `/Game/Roberts_stuff/LevelPrototyping/Interactable/Door/BP_DoorFrame.Enemy's Dead?` false _returnvalue)))

(fn `UserConstructionScript`)