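; BP_Rifle is a pickup hitscan rifle that equips itself on an overlapping BP_FirstPersonCharacter and disables its mesh collision.
; FireShot line-traces on the Visibility channel from the owner's eye viewpoint out to Range, with debug drawing.
; On an actor hit it applies Damage, decrements Ammo and spawns sparks at the impact; misses use no ammo, and Ammo is never checked.
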(event `FireShot`
  (bind (_outlocation _outrotation) (`self.GetActorEyesViewPoint` (`self.OwnerCharacter`)))
  (bind _outhit (`KismetSystemLibrary.LineTraceSingle` :`Start` _outlocation :`End` (+ (* (`KismetMathLibrary.GetForwardVector` _outrotation) (`self.Range`)) _outlocation) :`TraceChannel` "TraceTypeQuery1" :`DrawDebugType` "ForDuration"))
  (bind (_bblockinghit _binitialoverlap _time _distance _location _impactpoint _normal _impactnormal _physmat _hitactor) (`GameplayStatics.BreakHitResult` _outhit))
  (`/Engine/EditorBlueprintResources/StandardMacros.IsValid` _hitactor
    (:`Is Valid`
      (if true
        (`GameplayStatics.ApplyDamage` _hitactor (`self.Damage`) (`Pawn.GetController` (`self.OwnerCharacter`)) self)
        (set `self.Ammo` (- (`self.Ammo`) 1))
        (`GameplayStatics.SpawnEmitterAtLocation` "/Game/Roberts_stuff/StarterContent/Particles/P_Sparks.P_Sparks" _impactpoint (`KismetMathLibrary.MakeRotFromX` _impactnormal))))))

(event `self.ReceiveActorBeginOverlap`
  (params (OtherActor :type "Actor Object Reference"))
  (bind _asbp_first_person_character (cast `/Game/FirstPerson/Blueprints/BP_FirstPersonCharacter` OtherActor))
  (`/Game/FirstPerson/Blueprints/BP_FirstPersonCharacter.EquipWeapon` _asbp_first_person_character self)
  (`PrimitiveComponent.SetCollisionEnabled` (`self.Rifle`) "NoCollision"))

(fn `UserConstructionScript`)